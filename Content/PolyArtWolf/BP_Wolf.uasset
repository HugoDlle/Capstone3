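; BP_Wolf is a wolf that the player can talk to through a line-by-line dialogue.
; Overlapping its TriggerZone with BP_ThirdPersonCharacter shows a hint widget.
; Each Talk call clears the hint, advances DialogueIndex and shows that Dialogue entry in a dialogue widget, created when none is valid.
; When the lines run out, it reactivates the passed character's movement and removes the dialogue widget.
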(event OnComponentBeginOverlap(TriggerZone)
  (params (OverlappedComponent :type Primitive%20Component%20Object%20Reference) (OtherActor :type Actor%20Object%20Reference) (OtherComp :type Primitive%20Component%20Object%20Reference) (OtherBodyIndex :type Integer) (bFromSweep :type Boolean) (SweepResult :type Hit%20Result%20Structure%20%28by%20ref%29))
  (Utilities|Casting|CastToBP_ThirdPersonCharacter OtherActor)
  (bind _returnvalue (UserInterface|CreateWidget "/Game/Map/Level_Chapitre1/WBP_Hint.WBP_Hint_C" (Game|GetPlayerController 0)))
  (bind _output_get (Variables|Default|SetHintWBP _returnvalue))
  (UserInterface|Viewport|AddtoViewport _output_get 0))

(event EventTalk
  (params (Character%20Ref :type BP%20Third%20Person%20Character%20Object%20Reference))
  (bind _hintwbp (Variables|Default|GetHintWBP))
  (Utilities|IsValid _hintwbp
    (:Is%20Valid
      (Widget|RemovefromParent _hintwbp))
    (:Is%20Not%20Valid
      _))
  (Math|Integer|IncrementInt (Variables|Default|GetDialogue%20Index)
    (:%20%20
      (if (> (Utilities|Array|Length (Variables|Default|GetDialogue)) (Variables|Default|GetDialogue%20Index))
        (Variables|Default|GetDialogue%20Widget
          (:then
            _)
          (:else
            (bind _returnvalue (UserInterface|CreateWidget "/Game/Map/Level_Chapitre1/WBP_Dialogue.WBP_Dialogue_C" (Game|GetPlayerController 0) Character%20Ref))
            (bind _output_get (Variables|Default|SetDialogue%20Widget _returnvalue))
            (UserInterface|Viewport|AddtoViewport _output_get 0)))
        (Rendering|Components|TextRender|SetText (Variables|/Game/Map/Level_Chapitre1/WBP_Dialogue.WBP_Dialogue_C|GetDialogue_Box (Variables|Default|GetDialogue%20Widget)) (Utilities|Array|Get(acopy) (Variables|Default|GetDialogue) (Variables|Default|GetDialogue%20Index)))
        (else
          (Components|Activation|SetActive (Variables|/Script/Engine.Character|GetCharacterMovement Character%20Ref) true false)
          (Widget|RemovefromParent (Variables|Default|GetDialogue%20Widget)))))))

(fn ConstructionScript)