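; Rope Blueprint that builds a segmented mesh along its Rope spline in the construction script, with no active runtime logic.
; It multiplies SectionLength by the actor's X scale, then divides the spline length by it to set the segment count.
; Each segment is an added spline mesh component fitted between local-space spline points, with tangents clamped to the section length to match each short piece.
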(event EventBeginPlay)

(event Collision|EventActorBeginOverlap
  (params (OtherActor :type Actor%20Object%20Reference)))

(event EventTick
  (params (DeltaSeconds :type Float%20%28single-precision%29)))

(fn ConstructionScript
  (bind _rope (Variables|Default|GetRope))
  (bind _output_get (Variables|Default|SetSectionLength (* (.x (Transformation|GetActorScale3D)) (Variables|Default|GetSectionLength))))
  (for _index (range 0 (Math|Float|Truncate (/ (Spline|GetSplineLength (Variables|Default|GetRope)) (Variables|Default|GetSectionLength))))
    (bind _returnvalue (AddComponent|AddSplineMeshComponent false))
    (SplineMesh|SetStartandEnd _returnvalue (Spline|GetLocationatDistanceAlongSpline _rope (* _index (Variables|Default|GetSectionLength)) "Local") (Math|Vector|ClampVectorSize (Spline|GetTangentatDistanceAlongSpline _rope (* _index (Variables|Default|GetSectionLength)) "Local") 0.0 _output_get) (Spline|GetLocationatDistanceAlongSpline _rope (+ (* _index (Variables|Default|GetSectionLength)) (Variables|Default|GetSectionLength)) "Local") (Math|Vector|ClampVectorSize (Spline|GetTangentatDistanceAlongSpline _rope (+ (* _index (Variables|Default|GetSectionLength)) (Variables|Default|GetSectionLength)) "Local") 0.0 _output_get) true :!class /Script/Engine.SplineMeshComponent)))