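; BP_Boss is a boss enemy that attacks the player in range and can be defeated by dashing into it.
; A detection sphere sets the attacking state unless stunned, letting axe overlaps kill the player.
; Dashing into the mesh spends a stun charge with timed recovery, or flags death once none remain.
; The mesh starts in single-animation mode until SwitchToABP hands it to the ABP_BlackKnight Animation Blueprint.
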(event OnComponentBeginOverlap(Sphere)
  (params (OverlappedComponent :type Primitive%20Component%20Object%20Reference) (OtherActor :type Actor%20Object%20Reference) (OtherComp :type Primitive%20Component%20Object%20Reference) (OtherBodyIndex :type Integer) (bFromSweep :type Boolean) (SweepResult :type Hit%20Result%20Structure%20%28by%20ref%29))
  ;[0 1 0] Detect player
  (Utilities|Casting|CastToBP_ThirdPersonCharacter OtherActor)
  (if (not (Variables|Default|Getis%20Stun))
    (Variables|Default|Setis%20Attacking true)))

(event OnComponentEndOverlap(Sphere)
  (params (OverlappedComponent :type Primitive%20Component%20Object%20Reference) (OtherActor :type Actor%20Object%20Reference) (OtherComp :type Primitive%20Component%20Object%20Reference) (OtherBodyIndex :type Integer))
  ;[0 1 0] Detect player
  (Utilities|Casting|CastToBP_ThirdPersonCharacter OtherActor)
  (Variables|Default|Setis%20Attacking false))

(event OnComponentBeginOverlap(Axe)
  (params (OverlappedComponent :type Primitive%20Component%20Object%20Reference) (OtherActor :type Actor%20Object%20Reference) (OtherComp :type Primitive%20Component%20Object%20Reference) (OtherBodyIndex :type Integer) (bFromSweep :type Boolean) (SweepResult :type Hit%20Result%20Structure%20%28by%20ref%29))
  ;[0 1 0] Kill Player
  (bind _asbp_third_person_character (Utilities|Casting|CastToBP_ThirdPersonCharacter OtherActor))
  (if (Variables|Default|Getis%20Attacking)
    (Variables|/Game/Player/Blueprints/BP_ThirdPersonCharacter.BP_ThirdPersonCharacter_C|SetIsDead _asbp_third_person_character true)
    (Default|PlayerDeathLogic _asbp_third_person_character)))

(event OnComponentBeginOverlap(Mesh)
  (params (OverlappedComponent :type Primitive%20Component%20Object%20Reference) (OtherActor :type Actor%20Object%20Reference) (OtherComp :type Primitive%20Component%20Object%20Reference) (OtherBodyIndex :type Integer) (bFromSweep :type Boolean) (SweepResult :type Hit%20Result%20Structure%20%28by%20ref%29))
  ;[0 1 0] Boss Death Logic
  (bind _asbp_third_person_character (Utilities|Casting|CastToBP_ThirdPersonCharacter OtherActor))
  (if (not (Variables|Default|Getis%20Stun))
    (if (Variables|/Game/Player/Blueprints/BP_ThirdPersonCharacter.BP_ThirdPersonCharacter_C|GetisDashing _asbp_third_person_character)
      (if (> (Variables|Default|GetStun%20Before%20Break) 0)
        (Variables|Default|Setis%20Stun true)
        (Math|Integer|DecrementInt (Variables|Default|GetStun%20Before%20Break)
          (:%20%20
            (CallFunction|SetRecoveryTimer 1.5)))
        (else
          (Variables|Default|SetIs%20Dead true))))))

(event Custom|Switch%20To%20ABP
  ;[0 1 0] set animation mode
  (Components|Animation|SetAnimationMode (Variables|Character|GetMesh) "AnimationBlueprint" true)
  (Class|SkeletalMeshComponent|SetAnimClass (Variables|Character|GetMesh) "/Game/IA/Boss/ABP_BlackKnight.ABP_BlackKnight_C"))

(event Custom|Set%20Recovery%20Timer
  (params (Recovery%20Timer :type Float%20%28double-precision%29))
  ;[0 1 0] Recovery Timer
  (Utilities|FlowControl|Delay Recovery%20Timer)
  (Variables|Default|Setis%20Stun false))

(event EventBeginPlay
  ;[0 1 0] set animation mode
  (Components|Animation|SetAnimationMode (Variables|Character|GetMesh) "AnimationSingleNode" true)
  (Components|Animation|SetAnimation (Variables|Character|GetMesh) 0))

(fn ConstructionScript)