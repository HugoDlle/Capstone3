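; BP_IADragon is a dragon enemy that either dies or kills the player on contact.
; A capsule overlap casts the other actor to BP_ThirdPersonCharacter and checks whether it is dashing.
; A dashing player gets their dash reset, while the dragon stops moving, loses capsule collision and flags itself dead.
; Otherwise, the player is flagged dead and their death logic runs.
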(event OnComponentBeginOverlap(CapsuleComponent)
  (params (OverlappedComponent :type Primitive%20Component%20Object%20Reference) (OtherActor :type Actor%20Object%20Reference) (OtherComp :type Primitive%20Component%20Object%20Reference) (OtherBodyIndex :type Integer) (bFromSweep :type Boolean) (SweepResult :type Hit%20Result%20Structure%20%28by%20ref%29))
  ;[0.013 1 0] Enemy Damage Logic
  (bind _asbp_third_person_character (Utilities|Casting|CastToBP_ThirdPersonCharacter OtherActor))
  (Utilities|IsValid _asbp_third_person_character
    (:Is%20Valid
      (if (Variables|/Game/Player/Blueprints/BP_ThirdPersonCharacter.BP_ThirdPersonCharacter_C|GetisDashing _asbp_third_person_character)
        (Default|ResetPlayerDash _asbp_third_person_character)
        (Pawn|Components|CharacterMovement|DisableMovement (Variables|Character|GetCharacterMovement))
        (Collision|SetCollisionEnabled (Variables|Default|GetCapsuleComponent) "NoCollision")
        (Variables|Default|SetIs%20Dead%20? true)
        (else
          (Variables|/Game/Player/Blueprints/BP_ThirdPersonCharacter.BP_ThirdPersonCharacter_C|SetIsDead _asbp_third_person_character true)
          (Default|PlayerDeathLogic _asbp_third_person_character))))))

(fn ConstructionScript
  (|CallParentFunction))