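; BP_Play_Cinematic is a one-shot trigger box that plays a level sequence cinematic when the third-person character overlaps it.
; It disables the player's character movement, starts the sequence, and polls with a looping timer until playback stops.
; It then sets the Wolf to a seated idle animation at a hardcoded transform, restores player movement and destroys itself.
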(event OnComponentBeginOverlap(Box)
  (params (OverlappedComponent :type Primitive%20Component%20Object%20Reference) (OtherActor :type Actor%20Object%20Reference) (OtherComp :type Primitive%20Component%20Object%20Reference) (OtherBodyIndex :type Integer) (bFromSweep :type Boolean) (SweepResult :type Hit%20Result%20Structure%20%28by%20ref%29))
  (bind _asbp_third_person_character (Utilities|Casting|CastToBP_ThirdPersonCharacter OtherActor))
  (bind _output_get (Variables|Default|SetPlayer _asbp_third_person_character))
  (Components|Activation|SetActive (Variables|/Script/Engine.Character|GetCharacterMovement _output_get) false false)
  (bind _outactor (Sequencer|Player|CreateLevelSequencePlayer (Variables|Default|GetLVS_sequence)))
  (Sequencer|Player|Play (Variables|/Script/LevelSequence.LevelSequenceActor|GetSequencePlayer _outactor) :!class /Script/MovieScene.MovieSceneSequencePlayer)
  (Utilities|Time|SetTimerbyEvent (delegate Custom|Check%20playing) 0.05 true))

(event Custom|Check%20playing
  (bind _wolf (Variables|Default|GetWolf))
  (if (not (Audio|Components|Audio|IsPlaying (Variables|/Script/LevelSequence.LevelSequenceActor|GetSequencePlayer (stale OnComponentBeginOverlap(Box) _outactor))))
    (Components|Animation|SetAnimation (Variables|/Game/PolyArtWolf/BP_Wolf.BP_Wolf_C|GetSkeletalMesh _wolf) "/Game/PolyArtWolf/Animations/Common/Wolf_C_Seat_Idle.Wolf_C_Seat_Idle")
    (Transformation|SetActorTransform _wolf (Math|Transform|MakeTransform "495.339752,-1410.961914,455.770752" "0.000000,86.721985,0.000000" "1.000000,1.000000,1.000000"))
    (Components|Activation|SetActive (Variables|/Script/Engine.Character|GetCharacterMovement (Variables|Default|GetPlayer)) true false)
    (Actor|DestroyActor)))

(fn ConstructionScript)